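; Zombie enemy character that runs a behavior tree, detects the player and supplies spline patrol helpers.
; Physical animation drives simulated bodies below a bone for physically reactive motion.
; A looping timer sphere-overlaps for the shooter character to set DetectPlayer, while helpers provide patrol points and randomized wait times.
; Once accumulated damage reaches HealthCount, it simulates the body below root, stops AI and movement, and disables capsule collision.
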(event Custom|ReceiveDamage
  (params (Counter :type Integer))
  (bind _self self)
  (bind _returnvalue (AI|GetAIController _self))
  (bind _braincomponent (Variables|/Script/AIModule.AIController|GetBrainComponent _returnvalue))
  ;[0.3987 1 0.8593] Recieve Damage
  (Variables|Non-Editable|SetCounter (+ (Variables|Non-Editable|GetCounter) Counter))
  (if (>= (Variables|Non-Editable|GetCounter) (Variables|Settings|GetHealthCount))
    (Utilities|FlowControl|DoOnce false
      (:Completed
        (Class|PhysicalAnimationComponent|ApplyPhysicalAnimationSettingsBelow (Variables|Default|GetPhysicalAnimation) (Variables|Non-Editable|GetBone) (Utilities|Struct|MakePhysicalAnimationData true 1001.0 1e+02 1e+03 1e+02) false)
        (Class|SkeletalMeshComponent|SetAllBodiesBelowSimulatePhysics (Variables|Character|GetMesh) (Utilities|Name|MakeLiteralName "root") true false)
        (Class|PhysicalAnimationComponent|SetSkeletalMeshComponent (Variables|Default|GetPhysicalAnimation))
        (Utilities|IsValid _braincomponent
          (:Is%20Valid
            (AI|Logic|StopLogic _braincomponent ""))
          (:Is%20Not%20Valid
            _))
        (AI|Navigation|StopMovement _returnvalue)
        (Collision|SetCollisionEnabled (Variables|Collision|GetCapsuleComponent) "NoCollision")))))

(event Custom|AIPerception
  ;[0.513 0.6066 1] AIPerception
  (bind _returnvalue (Collision|SphereOverlapActors (Transformation|GetActorLocation) (Variables|Settings|GetPlayerDetectionRadius) (Utilities|Array|MakeArray "ObjectTypeQuery3") "/Game/TPTR_V4/Character/Blueprints/MainCharacter_Shooter.MainCharacter_Shooter_C"))
  (if _returnvalue
    (Variables|Non-Editable|SetDetectPlayer true)
    (else
      (Variables|Non-Editable|SetDetectPlayer false))))

(event EventBeginPlay
  (Class|PhysicalAnimationComponent|SetSkeletalMeshComponent (Variables|Default|GetPhysicalAnimation) (Variables|Character|GetMesh))
  (Class|PhysicalAnimationComponent|ApplyPhysicalAnimationSettingsBelow (Variables|Default|GetPhysicalAnimation) (Variables|Non-Editable|GetBone) (Utilities|Struct|MakePhysicalAnimationData false 2e+02 2e+02 1.11e+03 1e+02 1e+03 1e+04) true)
  (Class|SkeletalMeshComponent|SetAllBodiesBelowSimulatePhysics (Variables|Character|GetMesh) (Variables|Non-Editable|GetBone) true false)
  (Utilities|Time|SetTimerbyEvent (delegate Custom|AIPerception) (Variables|Settings|GetAIPerceptionFreq) true)
  (AI|RunBehaviorTree (AI|GetAIController self) "/Game/Enemy/BT_Zombie.BT_Zombie"))

(fn ConstructionScript)

(fn GetPatrolWaitTime
  (bind _randomdeviation (Variables|Settings|Patrol|GetRandomDeviation))
  (return (+ (Variables|Settings|Patrol|GetPatrolWaitTime) (Math|Random|RandomFloatinRange (* _randomdeviation -1.0) _randomdeviation))))

(fn GetTargetPatrolPoint
  (return (Spline|GetLocationatSplinePoint (Variables|/Game/Enemy/BP_PatrolsSpline.BP_PatrolsSpline_C|GetSpline (Variables|Settings|GetPatrolActor)) (Variables|Non-Editable|GetPatrolIndex) "World")))

(fn SetNextPatrolPoint
  (bind _patrolactor (Variables|Settings|GetPatrolActor)
    (:then
      (if (< (Variables|Non-Editable|GetPatrolIndex) (- (Spline|GetNumberOfSplinePoints (Variables|/Game/Enemy/BP_PatrolsSpline.BP_PatrolsSpline_C|GetSpline _patrolactor)) 1))
        (Math|Integer|IncrementInt (Variables|Non-Editable|GetPatrolIndex))
        (else
          (Variables|Non-Editable|SetPatrolIndex 0))))
    (:else)))