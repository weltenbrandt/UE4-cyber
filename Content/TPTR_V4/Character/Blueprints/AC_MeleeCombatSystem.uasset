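; Actor component that handles melee attacks and blocking for the shooter main character, using player 0's mesh cached at BeginPlay.
; Montages come from a single hard-coded row in the DT_MeleeCombat data table.
; Each attack plays the next montage in the row's Attack array, wrapping after the last, with no timed combo reset.
; Blocking plays the row's Block montage and stops it with a short blend-out.
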(event EventBeginPlay
  (bind _asmain_character_shooter (Utilities|Casting|CastToMainCharacter_Shooter (Game|GetPlayerCharacter 0)))
  (Variables|Default|SetMesh (Variables|/Script/Engine.Character|GetMesh _asmain_character_shooter)))

(event EventTick
  (params (DeltaSeconds :type Float%20%28single-precision%29)))

(fn MeleeAttack
  (bind _out_row (CallFunction|GetCurrentCombatData))
  (bind _attack (Utilities|Struct|BreakFMeleeCombat _out_row))
  (Utilities|IsValid (Utilities|Array|Get(acopy) _attack (Variables|Default|GetMontageIndex))
    (:Is%20Valid
      (Animation|Montage|MontagePlay (Components|SkeletalMesh|GetAnimInstance (Variables|Default|GetMesh)) (Utilities|Array|Get(acopy) _attack (Variables|Default|GetMontageIndex)) 1.0 "MontageLength" 0.0 true)
      (if (== (Variables|Default|GetMontageIndex) (Utilities|Array|LastIndex _attack))
        (Variables|Default|SetMontageIndex 0)
        (else
          (Math|Integer|IncrementInt (Variables|Default|GetMontageIndex)))))))

(fn GetCurrentCombatData
  (bind _returnvalue (Utilities|GetDataTableRow "/Game/TPTR_V4/Character/Blueprints/DT_MeleeCombat.DT_MeleeCombat" "NewRow")
    (:then
      (return _returnvalue))))

(fn StartBlock
  (bind _out_row (CallFunction|GetCurrentCombatData))
  (bind _block (Utilities|Struct|BreakFMeleeCombat _out_row))
  (Utilities|IsValid _block
    (:Is%20Valid
      (Animation|Montage|MontagePlay (Components|SkeletalMesh|GetAnimInstance (Variables|Default|GetMesh)) _block 1.0 "MontageLength" 0.0 true))))

(fn StopBlock
  (bind _out_row (CallFunction|GetCurrentCombatData))
  (bind _block (Utilities|Struct|BreakFMeleeCombat _out_row))
  (Utilities|IsValid _block
    (:Is%20Valid
      (Animation|Montage|MontageStop (Components|SkeletalMesh|GetAnimInstance (Variables|Default|GetMesh)) 0.25 _block))))