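; Bullet projectile for the shooter character, taking its mesh, transform, speed and range from the current weapon and visible only if slow-mo is on at spawn.
; FireBullet line-traces between successive frame positions until a hit, with a range-based timeout destroying the bullet.
; Tagged glass breaks through the character and lets non-shotgun bullets continue.
; Other hits destroy the bullet, giving zombies an impulse and equal damage for head or body.
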(event Custom|Fire%20Bullet
  (bind _weapon_shot_from (Variables|Default|GetWeapon%20Shot%20From))
  (Utilities|FlowControl|Sequence
    (:then_0
      ;[0 0 0] Get the initial location of the projectile
      (Variables|Default|SetStart%20Trace (Transformation|GetActorLocation) :!label _label)
      ;[0 0 0] After a single frame has passed, get the location once again
      (Utilities|FlowControl|Delay 0.0)
      (Variables|Default|SetEnd%20Trace (Transformation|GetActorLocation))
      ;[0 0 0] Create a line trace based on those two points, and store the out hit values
      (bind (_outhit _returnvalue) (Collision|LineTraceByChannel (Variables|Default|GetStart%20Trace) (Variables|Default|GetEnd%20Trace) "TraceTypeQuery1" false 0 "ForDuration" true "(R=1.000000,G=0.000000,B=0.000000,A=1.000000)" "(R=0.000000,G=1.000000,B=0.000000,A=1.000000)" 1.0))
      (Variables|Default|SetOut%20Hit _outhit)
      (bind _output_get (Variables|Default|SetHit? _returnvalue))
      ;[0 0 0] If there is no hit, repeat the process
      (if _output_get
        ;[0 0 0] If there is a hit, check to see if it's glass. If it is glass, then destroy it and then repeate the process as if the bullet never hit anything.
        (Variables|Default|SetHit%20Location (.Location (Collision|BreakHitResult (Variables|Default|GetOut%20Hit))))
        (if (not (Components|ComponentHasTag (.HitComponent (Collision|BreakHitResult (Variables|Default|GetOut%20Hit))) "Glass"))
          (Actor|DestroyActor)
          (CallFunction|HitAICharacter)
          (else
            (CallFunction|DestroyGlass)
            (goto _label)))
        (else
          (goto _label))))
    (:then_1
      (Utilities|FlowControl|Delay (/ (Variables|/Game/TPTR_V4/Weapons/Weapon_Parent.Weapon_Parent_C|GetBullet:%20Max%20Travel%20Distance%20[in%20Meters] _weapon_shot_from) (Variables|/Game/TPTR_V4/Weapons/Weapon_Parent.Weapon_Parent_C|GetBullet:%20Speed%20[in%20Meters/sec] _weapon_shot_from)))
      (Actor|DestroyActor))))

(event EventBeginPlay
  (bind _asmain_character_shooter (Utilities|Casting|CastToMainCharacter_Shooter (Game|GetPlayerCharacter 0)))
  ;[0 0 0] This is were the bullet properties are established, based on the character's current weapon.
  (Rendering|SetVisibility (Variables|Default|GetSphere) (Variables|/Game/TPTR_V4/Character/Blueprints/MainCharacter_Shooter.MainCharacter_Shooter_C|GetSlowMo%20On _asmain_character_shooter) false)
  (Variables|Default|SetWeapon%20Shot%20From (Variables|/Game/TPTR_V4/Character/Blueprints/MainCharacter_Shooter.MainCharacter_Shooter_C|GetWeapon _asmain_character_shooter))
  (Components|StaticMesh|SetStaticMesh (Variables|Default|GetSphere) (Variables|/Game/TPTR_V4/Weapons/Weapon_Parent.Weapon_Parent_C|GetBullet:%20Static%20Mesh (Variables|Default|GetWeapon%20Shot%20From)))
  (Transformation|SetWorldScale3D (Variables|Default|GetSphere) (Variables|/Game/TPTR_V4/Weapons/Weapon_Parent.Weapon_Parent_C|GetBullet:%20Scale (Variables|Default|GetWeapon%20Shot%20From)))
  (Transformation|SetRelativeRotation (Variables|Default|GetSphere) (Variables|/Game/TPTR_V4/Weapons/Weapon_Parent.Weapon_Parent_C|GetBullet:%20Rotation (Variables|Default|GetWeapon%20Shot%20From)) false false)
  (Game|Components|ProjectileMovement|SetVelocityinLocalSpace (Variables|Default|GetProjectileMovement) (Math|Vector|MakeVector (Variables|/Game/TPTR_V4/Weapons/Weapon_Parent.Weapon_Parent_C|GetBullet:%20Speed%20[in%20Meters/sec] (Variables|Default|GetWeapon%20Shot%20From)) 0.0 0.0))
  (Variables|/Script/Engine.ProjectileMovementComponent|SetProjectileGravityScale (Variables|Default|GetProjectileMovement) 1.0))

(fn ConstructionScript)

(fn DestroyGlass
  (bind _out_hit (Variables|Default|GetOut%20Hit))
  (bind (_bblockinghit _binitialoverlap _time _distance _location _impactpoint _normal _impactnormal _physmat _hitactor _hitcomponent _hitbonename _hititem _faceindex _tracestart) (Collision|BreakHitResult _out_hit))
  (bind _assa_dest_glass_panel (Utilities|Casting|CastToSA_Dest_GlassPanel _hitactor))
  (Variables|Default|SetGlassObject _assa_dest_glass_panel)
  (bind _asmain_character_shooter (Utilities|Casting|CastToMainCharacter_Shooter (Game|GetPlayerCharacter 0)))
  (Default|MakeGlassBreak _asmain_character_shooter (Math|Rotator|FindLookatRotation _tracestart (Variables|Default|GetHit%20Location)) (Variables|Default|GetHit%20Location) (Variables|Default|GetGlassObject) true)
  (if (Variables|/Game/TPTR_V4/Weapons/Weapon_Parent.Weapon_Parent_C|GetShotgun:%20Is%20Shotgun? (Variables|Default|GetWeapon%20Shot%20From))
    (Actor|DestroyActor)
    (else
      (Variables|Default|SetStart%20Trace (Variables|Default|GetHit%20Location)))))

(fn HitAICharacter
  (bind _out_hit (Variables|Default|GetOut%20Hit))
  (bind (_bblockinghit _binitialoverlap _time _distance _location _impactpoint _normal _impactnormal _physmat _hitactor _hitcomponent _hitbonename) (Collision|BreakHitResult _out_hit))
  ;[0 0 0] This Function will handle the interactions that take place between the AI and the weapons. The if statement will handle component tags, and that's how you'll be able to multiply the damage value of the ebullet, based on what's being hit (head, or body in this case).
  (bind _asbp_zombie (Utilities|Casting|CastToBP_Zombie _hitactor))
  (bind _output_get (LocalVariables|Setlocal%20AI%20Char _asbp_zombie))
  (Physics|AddImpulse (Variables|/Script/Engine.Character|GetMesh _output_get) (* (Transformation|GetActorLocation (Game|GetPlayerCharacter 0)) -1e+01) _hitbonename false)
  (if (Components|ComponentHasTag (.HitComponent (Collision|BreakHitResult (Variables|Default|GetOut%20Hit))) "AI_Head")
    (Default|ReceiveDamage (LocalVariables|Getlocal%20AI%20Char) 1)
    (else
      (Default|ReceiveDamage (LocalVariables|Getlocal%20AI%20Char) 1))))